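; Game mode for the FeeFiFoFum game that owns the pause menu.
; On BeginPlay it creates the MenuHUD widget, adds it to the viewport and keeps it hidden.
; Pause and Resume functions toggle the game's paused state and show or hide that menu to match.
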(event EventBeginPlay
  (bind _returnvalue (UserInterface|CreateWidget "/Game/Blueprints/MenuHUD.MenuHUD_C"))
  (bind _output_get (Variables|Default|SetMenu _returnvalue))
  (UserInterface|Viewport|AddtoViewport _output_get 0)
  (Widget|SetVisibility _output_get "Hidden")
  (Development|PrintString "Created"))

(fn ConstructionScript)

(fn Resume
  (Game|SetGamePaused false)
  (Widget|SetVisibility (Variables|Default|GetMenu) "Hidden"))

(fn Pause
  (Game|SetGamePaused true)
  (Widget|SetVisibility (Variables|Default|GetMenu) "Visible"))