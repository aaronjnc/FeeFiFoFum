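; BP_Throw is an actor that launches a passed-in character from its own position.
; Its Throw function moves the character to the actor's location and adds a capsule impulse along the actor's forward vector, scaled by Velocity.
; The SetActorRotation call there reapplies the actor's own rotation, leaving the character's untouched.
; When a BP_FirstPersonCharacter stops overlapping the Box, it calls Pause on BP_FeeFiFoFumGameMode.
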(event OnComponentEndOverlap(Box)
  (params (OverlappedComponent :type Primitive%20Component%20Object%20Reference) (OtherActor :type Actor%20Object%20Reference) (OtherComp :type Primitive%20Component%20Object%20Reference) (OtherBodyIndex :type Integer))
  (Utilities|Casting|CastToBP_FirstPersonCharacter OtherActor)
  (bind _asbp_fee_fi_fo_fum_game_mode (Utilities|Casting|CastToBP_FeeFiFoFumGameMode (Game|GetGameMode)))
  (Default|Pause _asbp_fee_fi_fo_fum_game_mode))

(fn ConstructionScript)

(fn Throw
  (params (Character :type BP%20First%20Person%20Character%20Object%20Reference))
  (bind _velocity (Variables|Default|GetVelocity))
  (Transformation|SetActorLocation Character (Transformation|GetActorLocation) false false)
  (Transformation|SetActorRotation (Transformation|GetActorRotation))
  (Physics|AddImpulse (Variables|/Script/Engine.Character|GetCapsuleComponent Character) (* (Math|Vector|GetForwardVector (Transformation|GetActorRotation)) (Math|Vector|MakeVector _velocity _velocity _velocity)) "None" false))