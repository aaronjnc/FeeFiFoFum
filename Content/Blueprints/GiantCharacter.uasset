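; Giant enemy character that patrols PatrolPoint actors and pursues the first-person player once spotted.
; GiantPatrol picks each destination for a looping AI move with a short pause, while Tick eases yaw using the current path's first point.
; An overlap with clear line of sight halts it, then after PursueTime it chases, printing "Kill" when the move finishes.
; The player leaving the overlap resets detection and resumes patrol.
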(event EventBeginPlay
  (bind _outactors (Actor|GetAllActorsOfClass "/Script/FeeFiFoFum.PatrolPoint"))
  (Variables|/Script/FeeFiFoFum.GiantPatrol|SetPatrolPoints (Variables|Default|GetGiantPatrol) _outactors)
  (Utilities|MovetoLocation :!label _label)
  (goto _label))

(event Collision|EventActorBeginOverlap
  (params (OtherActor :type Actor%20Object%20Reference))
  (bind _outhit (Collision|LineTraceByChannel (Transformation|GetActorLocation) (Transformation|GetActorLocation OtherActor) "TraceTypeQuery1" false 0 "None"))
  (bind _asbp_first_person_character (Utilities|Casting|CastToBP_FirstPersonCharacter (.HitActor (Collision|BreakHitResult _outhit))))
  (Variables|Default|SetPlayer _asbp_first_person_character)
  (Variables|Default|SetSpotted true)
  (Components|Movement|StopMovementImmediately (Variables|Character|GetCharacterMovement)))

(event EventTick
  (params (DeltaSeconds :type Float%20%28single-precision%29))
  (Utilities|IsValid (Variables|Default|GetNextPoint)
    (:Is%20Valid
      (CallFunction|Lookat DeltaSeconds)
      (if (Variables|Default|GetSpotted)
        (Variables|Default|SetTimeSinceSpotted (+ (Variables|Default|GetTimeSinceSpotted) DeltaSeconds))
        (if (and (>= (Variables|Default|GetTimeSinceSpotted) (Variables|Default|GetPursueTime)) (not (Variables|Default|GetPursuingPlayer)))
          (AI|AIMoveTo (AI|GetAIController self) "0, 0, 0" (Variables|Default|GetPlayer) 25.0 "Default" "Default" true true
            (:then
              (Variables|Default|SetPursuingPlayer true))
            (:OnMoveFinished
              (Development|PrintString "Kill"))))))))

(event Collision|EventActorEndOverlap
  (params (OtherActor :type Actor%20Object%20Reference))
  (Utilities|Casting|CastToBP_FirstPersonCharacter OtherActor)
  (Variables|Default|SetPursuingPlayer false)
  (Variables|Default|SetSpotted false)
  (Variables|Default|SetTimeSinceSpotted 0.0)
  (Utilities|MovetoLocation :!label _label)
  (goto _label))

(fn ConstructionScript)

(fn Lookat
  (params (DeltaTime :type Float%20%28double-precision%29))
  (bind _returnvalue (Transformation|GetActorRotation))
  (bind _self self)
  (bind (_roll _pitch) (Math|Rotator|BreakRotator _returnvalue))
  (bind _returnvalue_2 (AI|GetAIController _self))
  (bind _returnvalue_3 (Class|AIBlueprintHelperLibrary|GetCurrentPathPoints _returnvalue_2))
  (if (Utilities|Array|IsValidIndex _returnvalue_3)
    (Transformation|SetActorRotation (Math|Interpolation|RInterpTo _returnvalue (Math|Rotator|MakeRotator _roll _pitch (.Yaw (Math|Rotator|BreakRotator (Math|Rotator|FindLookatRotation (Utilities|Array|Get(acopy) _returnvalue_3) (Transformation|GetActorLocation))))) DeltaTime 2.0))))